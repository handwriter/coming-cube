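; BP_DeathWall is a wall hazard that reacts when the player touches it.
; On overlap with BP_Player it switches the Cube to MAT_Death and detaches the player's camera in world space.
; A DeathAnim event, not called here, loops scale translate and return through TranslatePositionComponent; its timers target an empty event, so the loop never waits.
; RandomScale holds only unused nodes.
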(event Custom|Death%20Anim
  (bind _translatepositioncomponent (Variables|Default|GetTranslatePositionComponent))
  (bind _translateseconds (Variables|/Game/Blueprints/TranslatePositionComponent.TranslatePositionComponent_C|GetTranslateSeconds _translatepositioncomponent))
  (Default|StartTranslate _translatepositioncomponent "0, 0, 0" "-1.000000, 0, 0" "0, 0, 0" :!label _label)
  (Utilities|Time|SetTimerbyEvent (delegate Custom|CustomEvent_0) _translateseconds)
  (Default|ReturnTranslate _translatepositioncomponent)
  (Utilities|Time|SetTimerbyEvent (delegate Custom|CustomEvent_0) _translateseconds)
  (goto _label))

(event Custom|CustomEvent_0)

(event EventBeginPlay)

(event Collision|EventActorBeginOverlap
  (params (OtherActor :type Actor%20Object%20Reference))
  (bind _asbp_player (Utilities|Casting|CastToBP_Player OtherActor))
  (Rendering|Material|SetMaterial (Variables|Default|GetCube) 0 "/Game/Materials/MAT_Death.MAT_Death")
  (Transformation|DetachFromComponent (Variables|/Game/Blueprints/BP_Player.BP_Player_C|GetCamera _asbp_player) "KeepWorld" "KeepWorld" "KeepWorld" true))

(event EventTick
  (params (DeltaSeconds :type Float%20%28single-precision%29)))

(fn ConstructionScript)