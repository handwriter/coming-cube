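; Scene component that slides its attach parent by a world-space location offset in timed steps, with reverse and stop events.
; StartTranslate derives step count and delta from TranslateSeconds and UpdPerSeconds, then a looping timer applies teleporting world offsets until the count is reached.
; ReturnTranslate flips the direction sign and reuses that setup, retracing only completed steps if interrupted.
; EndTranslate pauses the timer; the ScaleOffset input is unused.
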(event Custom|StartTranslate
  (params (Location%20Offset :type Vector) (Scale%20Offset :type Vector))
  ;[1 1 1] Translate Position Event
  (Variables|Default|SetParent (Transformation|GetAttachParent))
  (Variables|Default|SetLocalAxis 1.0)
  (Variables|Default|SetNeedIteration (Math|Float|Truncate (* (Variables|Default|GetTranslateSeconds) (Variables|Default|GetUpdPerSeconds))))
  (Variables|Default|SetCurrentIteration 0)
  (Variables|Default|SetObjectStartPosition (Transformation|GetWorldLocation (Variables|Default|GetParent)))
  (Variables|Default|SetDeltaOffset (/ (/ Location%20Offset (Variables|Default|GetTranslateSeconds)) (Variables|Default|GetUpdPerSeconds)))
  (bind _returnvalue (Utilities|Time|SetTimerbyEvent (delegate Custom|TranslatePositionIteration) (/ (Variables|Default|GetTranslateSeconds) (Variables|Default|GetUpdPerSeconds)) true))
  (Variables|Default|SetLocal%20Change%20Timer _returnvalue))

(event Custom|ReturnTranslate
  ;[1 1 1] Return To Start Position Event
  (Utilities|Time|PauseTimerbyHandle (Variables|Default|GetLocal%20Change%20Timer))
  (Variables|Default|SetLocalAxis -1.0)
  (if (>= (Variables|Default|GetCurrentIteration) (Variables|Default|GetNeedIteration))
    _
    (else
      (Variables|Default|SetNeedIteration (Variables|Default|GetCurrentIteration))))
  ;[1 1 1] Translate Position Event
  (Variables|Default|SetCurrentIteration 0)
  (Variables|Default|SetObjectStartPosition (Transformation|GetWorldLocation (Variables|Default|GetParent)))
  (Variables|Default|SetDeltaOffset (/ (/ (stale Custom|StartTranslate Location%20Offset) (Variables|Default|GetTranslateSeconds)) (Variables|Default|GetUpdPerSeconds)))
  (bind _returnvalue (Utilities|Time|SetTimerbyEvent (delegate Custom|TranslatePositionIteration) (/ (Variables|Default|GetTranslateSeconds) (Variables|Default|GetUpdPerSeconds)) true))
  (Variables|Default|SetLocal%20Change%20Timer _returnvalue))

(event Custom|TranslatePositionIteration
  ;[1 1 1] Translate Position Event
  (Math|Integer|IncrementInt (Variables|Default|GetCurrentIteration)
    (:%20%20
      (if (>= (Variables|Default|GetCurrentIteration) (Variables|Default|GetNeedIteration))
        (Utilities|Time|PauseTimerbyHandle (Variables|Default|GetLocal%20Change%20Timer))
        (Variables|Default|SetIsMoving false)
        (else
          (Transformation|AddWorldOffset (Variables|Default|GetParent) (* (Variables|Default|GetDeltaOffset) (Variables|Default|GetLocalAxis)) false true)
          (Variables|Default|SetIsMoving true))))))

(event Custom|End%20Translate
  ;[1 1 1] Outside End Translation Timer
  (Utilities|Time|PauseTimerbyHandle (Variables|Default|GetLocal%20Change%20Timer)))

(event EventBeginPlay)

(event EventTick
  (params (DeltaSeconds :type Float%20%28single-precision%29)))