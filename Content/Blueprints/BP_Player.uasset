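; Player pawn that moves forward continuously, steers sideways from input and stops on hitting a death wall.
; Tick pushes the mesh along local negative X, axis inputs shift the whole actor on world Y.
; Left and right key presses slide the camera sideways through a translate component, returning it on release.
; Overlapping BP_DeathWall zeroes speed, disables input, translates toward the wall's box center and prints a placeholder message.
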(event EventBeginPlay)

(event Collision|EventActorBeginOverlap
  (params (OtherActor :type Actor%20Object%20Reference))
  (bind _centertranslateplayer (Variables|Default|GetCenterTranslatePlayer))
  (bind _asbp_death_wall (Utilities|Casting|CastToBP_DeathWall OtherActor))
  ;[1 1 1] Translate te Center
  (Default|StartTranslate _centertranslateplayer (- (Transformation|GetWorldLocation (Variables|/Game/Blueprints/BP_DeathWall.BP_DeathWall_C|GetBox _asbp_death_wall)) (Transformation|GetWorldLocation (Variables|Default|GetStaticMesh))) "0, 0, 0" "0, 0, 0")
  (Variables|Default|SetSpeed 0.0)
  (Input|DisableInput 0)
  (while (Variables|/Game/Blueprints/TranslatePositionComponent.TranslatePositionComponent_C|GetIsMoving _centertranslateplayer)
    _)
  (Development|PrintString "Hello"))

(event EventTick
  (params (DeltaSeconds :type Float%20%28single-precision%29))
  ;[1 1 1] Moving Controller
  (Transformation|AddLocalOffset (Variables|Default|GetStaticMesh) (Math|Vector|MakeVector (* (* DeltaSeconds (Variables|Default|GetSpeed)) -1.0) 0.0 0.0) false true))

(event Input|ActionEvents|InputActionLeftKey
  (params (Key :type Key%20Structure :default "None"))
  (bind _cameratranslatepositioncomponent (Variables|Default|GetCameraTranslatePositionComponent))
  ;[1 1 1] Moving Controller
  (:Pressed
    (Variables|Default|SetCurrentAxis 1.0)
    (Default|StartTranslate _cameratranslatepositioncomponent (Math|Vector|MakeVector 0.0 (* (Variables|Default|GetCameraOffset) (Variables|Default|GetCurrentAxis)) 0.0) "0, 0, 0" "0, 0, 0"))
  (:Released
    (Variables|Default|SetCurrentAxis 0.0)
    (Default|ReturnTranslate _cameratranslatepositioncomponent)))

(event Input|ActionEvents|InputActionRightKey
  (params (Key :type Key%20Structure :default "None"))
  (bind _cameratranslatepositioncomponent (Variables|Default|GetCameraTranslatePositionComponent))
  ;[1 1 1] Moving Controller
  (:Pressed
    (Variables|Default|SetCurrentAxis -1.0)
    (Default|StartTranslate _cameratranslatepositioncomponent (Math|Vector|MakeVector 0.0 (* (Variables|Default|GetCameraOffset) (Variables|Default|GetCurrentAxis)) 0.0) "0, 0, 0" "0, 0, 0"))
  (:Released
    (Variables|Default|SetCurrentAxis 0.0)
    (Default|ReturnTranslate _cameratranslatepositioncomponent)))

(event Input|AxisEvents|InputAxisLeft
  (params (AxisValue :type Float%20%28single-precision%29))
  ;[1 1 1] Moving Controller
  (Transformation|AddActorWorldOffset (Math|Vector|MakeVector 0.0 (* AxisValue (* (Utilities|Time|GetWorldDeltaSeconds) (Variables|Default|GetAxisSpeed))) 0.0) false true))

(event Input|AxisEvents|InputAxisRight
  (params (AxisValue :type Float%20%28single-precision%29))
  ;[1 1 1] Moving Controller
  (Transformation|AddActorWorldOffset (Math|Vector|MakeVector 0.0 (* (* AxisValue (* (Utilities|Time|GetWorldDeltaSeconds) (Variables|Default|GetAxisSpeed))) -1.0) 0.0) false true))

(fn ConstructionScript)